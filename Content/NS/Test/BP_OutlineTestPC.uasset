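; Test player controller that highlights actors under the mouse cursor with an outline.
; On BeginPlay it shows the cursor and sets Game and UI input mode.
; Each tick it traces under the cursor on the Visibility channel and keeps hit actors implementing OutLineInterface.
; When that target changes on a blocking hit, interface messages turn the new outline on and the previous one off.
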(event `self.ReceiveBeginPlay`
  (set `self.bShowMouseCursor` true)
  (`WidgetBlueprintLibrary.SetInputMode_GameAndUIEx` self null "DoNotLock" false))

(event `self.ReceiveTick`
  (params (DeltaSeconds :type "Float (single-precision)"))
  (bind (_bblockinghit _binitialoverlap _time _distance _location _impactpoint _normal _impactnormal _physmat _hitactor) (`GameplayStatics.BreakHitResult` (`self.GetHitResultUnderCursorByChannel` "TraceTypeQuery1" false)))
  (if _bblockinghit
    (set `self.LastHitActor` (`self.CurrentHitActor`))
    (if (`KismetSystemLibrary.DoesImplementInterface` _hitactor "/Script/ProjectNS.OutLineInterface")
      (set `self.CurrentHitActor` _hitactor)
      (else
        (set `self.CurrentHitActor` null)))
    (if (!= (`self.CurrentHitActor`) (`self.LastHitActor`))
      (message `OutLineInterface.TurnOnOutline` (`self.CurrentHitActor`))
      (message `OutLineInterface.TurnOffOutline` (`self.LastHitActor`)))))

(fn `UserConstructionScript`)